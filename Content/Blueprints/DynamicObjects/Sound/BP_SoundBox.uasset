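; BP_SoundBox is a trigger volume that plays a configurable sound the first time the player enters it.
; A DoOnce on the player overlap creates and plays a 2D sound with the set cue, volume and pitch, persisting across level transitions.
; The construction script sizes the detection box on X and Z from a tile-based size and pixel-to-unit conversion, keeping Y depth fixed.
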(event `self.PlayerDetection.OnComponentBeginOverlap`
  (params (OverlappedComponent :type "PrimitiveComponent Object Reference") (OtherActor :type "Actor Object Reference") (OtherComp :type "PrimitiveComponent Object Reference") (OtherBodyIndex :type Integer) (bFromSweep :type Boolean) (SweepResult :type "HitResult Structure (by ref)"))
  (cast `/Game/Blueprints/Character/BP_Player` OtherActor)
  (`/Engine/EditorBlueprintResources/StandardMacros.DoOnce` false
    (:`Completed`
      (bind _returnvalue (`GameplayStatics.CreateSound2D` (`self.SoundQue`) (`self.Volume`) (`self.Pitch`) 0.0 null true))
      (`AudioComponent.Play` _returnvalue 0.0))))

(fn `UserConstructionScript`
  (bind (_returnvalue_x _returnvalue_y) (`KismetMathLibrary.BreakVector2D` (* (`self.DetectioonSize`) (`self.PixelPerTile`) (/ 1.0 (`self.PixelPerUnit`)) 0.5)))
  (`BoxComponent.SetBoxExtent` (`self.PlayerDetection`) (`KismetMathLibrary.MakeVector` _returnvalue_x 100.0 _returnvalue_y) true))