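; BP_Winning is a level-end trigger that plays the player's winning animation on overlap and is meant to change levels.
; Its box, sized in tiles by the construction script, disables player actions and jumps the animation state to winning.
; It then calls DestroyActor before the delayed level load, which flags route to Map_Level02 or Map_MainMenu, with a longer wait for credits.
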(event `self.PlayerDetection.OnComponentBeginOverlap`
  (params (OverlappedComponent :type "PrimitiveComponent Object Reference") (OtherActor :type "Actor Object Reference") (OtherComp :type "PrimitiveComponent Object Reference") (OtherBodyIndex :type Integer) (bFromSweep :type Boolean) (SweepResult :type "HitResult Structure (by ref)"))
  (bind _asbp_player (cast `/Game/Blueprints/Character/BP_Player` OtherActor))
  (set `/Game/Blueprints/Character/BP_Player.CanAct` false _asbp_player)
  (`PaperZDAnimInstance.JumpToNode` (`PaperZDCharacter.AnimInstance` _asbp_player) "JumpToWinning" "None")
  (`self.K2_DestroyActor`)
  (`KismetSystemLibrary.Delay` 1.0)
  (if (`self.NextLevel`)
    (`GameplayStatics.OpenLevel` "Map_Level02")
    (elif (`self.MainMenu`)
      (`GameplayStatics.OpenLevel` "Map_MainMenu")
      (elif (`self.Credits`)
        (`KismetSystemLibrary.Delay` 10.0)
        (`GameplayStatics.OpenLevel` "Map_MainMenu")))))

(fn `UserConstructionScript`
  (bind (_returnvalue_x _returnvalue_y) (`KismetMathLibrary.BreakVector2D` (* (`self.PlayeredetectionSize`) (`self.PixelPerTile`) (/ 1.0 (`self.PixelPerUnit`)) 0.5)))
  (`BoxComponent.SetBoxExtent` (`self.PlayerDetection`) (`KismetMathLibrary.MakeVector` _returnvalue_x 100.0 _returnvalue_y) true))