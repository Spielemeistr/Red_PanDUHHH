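; BP_MaskBase is a base collectable mask that grants the player an ability when picked up.
; On overlap with its collision box, it casts to BP_Player, calls AddAbility with its Ability value, then destroys itself.
; The construction script sets the flipbook sprite and sizes the box from a tile-based CollisionSize converted through pixel-per-tile and pixel-per-unit values, with fixed depth.
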(event `self.Collision.OnComponentBeginOverlap`
  (params (OverlappedComponent :type "PrimitiveComponent Object Reference") (OtherActor :type "Actor Object Reference") (OtherComp :type "PrimitiveComponent Object Reference") (OtherBodyIndex :type Integer) (bFromSweep :type Boolean) (SweepResult :type "HitResult Structure (by ref)"))
  (bind _asbp_player (cast `/Game/Blueprints/Character/BP_Player` OtherActor))
  (`/Game/Blueprints/Character/BP_Player.AddAbility` _asbp_player (`self.Ability`))
  (`self.K2_DestroyActor`))

(fn `UserConstructionScript`
  (bind (_returnvalue_x _returnvalue_y) (`KismetMathLibrary.BreakVector2D` (* (`self.CollisionSize`) (`self.PixelPerTile`) (`self.PixelPerUnit`) 0.5)))
  (`PaperFlipbookComponent.SetFlipbook` (`self.RenderComponent`) (`self.Flipbook`))
  (`BoxComponent.SetBoxExtent` (`self.Collision`) (`KismetMathLibrary.MakeVector` _returnvalue_x 100.0 _returnvalue_y) true))