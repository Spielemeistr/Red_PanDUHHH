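; Base spike trap for a 2D game that moves when the player enters its detection box and damages them on hit.
; A once-only trigger runs a timeline that offsets the actor in the XZ plane, optionally reversing after a delay to re-arm.
; A hit closes a gate that blocks pending returns until Reset restores position and trigger.
; The construction script sizes both boxes from tile and pixel units.
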(event `self.ReceiveBeginPlay`
  (set `self.StartLocation` (`self.K2_GetActorLocation`)))

(event `MoveSpike`
  (bind (_returnvalue_x _returnvalue_y _returnvalue_z) (`KismetMathLibrary.BreakVector` (`self.GetActorUpVector`)))
  (set `self.PlayForward` true)
  (`TimelineComponent.SetPlayRate` (`self.MoveSpikeValue`) (`self.PlaySpeed`))
  (bind (_direction _value) (`Timeline|MoveSpikeValue` :!via `PlayFromStart` :!label _label)
    (:`Update`
      (bind (_returnvalue_x_2 _returnvalue_y_2) (`KismetMathLibrary.BreakVector2D` (* _value (`self.MovementDistance`) (`self.MovementDirection`) _returnvalue_z)))
      (`self.K2_SetActorLocation` (+ (`self.StartLocation`) (`KismetMathLibrary.MakeVector` _returnvalue_x_2 0.0 _returnvalue_y_2))))
    (:`Finished`
      (if (`self.Return`)
        (if (`self.PlayForward`)
          (`KismetSystemLibrary.Delay` (`self.TransitionDelay`))
          (`/Engine/EditorBlueprintResources/StandardMacros.Gate` false :!label _label_2
            (:`Exit`
              (set `self.PlayForward` false)
              (goto _label :!via `ReverseFromEnd`)))
          (else
            (goto _label_3 :!via `Reset`)))))))

(event `self.HitBox.OnComponentBeginOverlap`
  (params (OverlappedComponent :type "PrimitiveComponent Object Reference") (OtherActor :type "Actor Object Reference") (OtherComp :type "PrimitiveComponent Object Reference") (OtherBodyIndex :type Integer) (bFromSweep :type Boolean) (SweepResult :type "HitResult Structure (by ref)"))
  (bind _asbp_player (cast `/Game/Blueprints/Character/BP_Player` OtherActor))
  (`/Game/Blueprints/Character/BP_Player.Damage` _asbp_player)
  (goto _label_2 :!via `Close`))

(event `self.PlayerDetection.OnComponentBeginOverlap`
  (params (OverlappedComponent :type "PrimitiveComponent Object Reference") (OtherActor :type "Actor Object Reference") (OtherComp :type "PrimitiveComponent Object Reference") (OtherBodyIndex :type Integer) (bFromSweep :type Boolean) (SweepResult :type "HitResult Structure (by ref)"))
  (cast `/Game/Blueprints/Character/BP_Player` OtherActor)
  (`/Engine/EditorBlueprintResources/StandardMacros.DoOnce` false :!label _label_3
    (:`Completed`
      (`self.MoveSpike`))))

(event `Reset`
  (`|ExecutionSequence`
    (:`then_0`
      (`KismetSystemLibrary.Delay` 0.5)
      (goto _label_2 :!via `Open`))
    (:`then_1`
      (`self.K2_SetActorLocation` (`self.StartLocation`))
      (goto _label_3 :!via `Reset`))))

(fn `UserConstructionScript`
  (bind (_playerdetectionoffset_x _playerdetectionoffset_y) (`KismetMathLibrary.BreakVector2D` (`self.PlayerDetectionOffset`)))
  (bind (_returnvalue_x _returnvalue_y) (`KismetMathLibrary.BreakVector2D` (* (`self.PlayerDetectionSize`) (`self.PixelPerTile`) (/ 1.0 (`self.PixelPerUnit`)) 0.5)))
  (bind (_returnvalue_x_2 _returnvalue_y_2) (`KismetMathLibrary.BreakVector2D` (* (`self.CollisionSize`) (`self.PixelPerTile`) (/ 1.0 (`self.PixelPerUnit`)) 0.5)))
  (`BoxComponent.SetBoxExtent` (`self.HitBox`) (`KismetMathLibrary.MakeVector` _returnvalue_x_2 100.0 _returnvalue_y_2) true)
  (`BoxComponent.SetBoxExtent` (`self.PlayerDetection`) (`KismetMathLibrary.MakeVector` _returnvalue_x 100.0 _returnvalue_y) true)
  (`SceneComponent.K2_AddLocalOffset` (`self.PlayerDetection`) (`KismetMathLibrary.MakeVector` _playerdetectionoffset_x 0.0 _playerdetectionoffset_y) false false))