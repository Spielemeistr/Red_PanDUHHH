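; BP_PlatformExploding is a one-shot exploding platform that plays a flipbook animation when BP_Player enters its PlayerDetection volume.
; The overlap passes a DoOnce that sets the flipbook play rate to PlaySpeed.
; Tick switches collision to overlap pawns at SetCollisionFalseFrame, letting them pass through, and stops playback on the last frame.
; The Reset event rewinds the flipbook, restores pawn blocking and re-arms the DoOnce.
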(event `self.ReceiveTick`
  (params (DeltaSeconds :type "Float (single-precision)"))
  (bind _rendercomponent (`self.RenderComponent`))
  (`parent.ReceiveTick` DeltaSeconds)
  (if (== (`PaperFlipbookComponent.GetPlaybackPositionInFrames` _rendercomponent) (- (`PaperFlipbookComponent.GetFlipbookLengthInFrames` _rendercomponent) 1))
    (`PaperFlipbookComponent.SetPlayRate` (`self.RenderComponent`) 0.0))
  (if (== (`PaperFlipbookComponent.GetPlaybackPositionInFrames` (`self.RenderComponent`)) (`self.SetCollisionFalseFrame`))
    (`PrimitiveComponent.SetCollisionResponseToChannel` (`self.Collision`) "ECC_Pawn" "ECR_Overlap")))

(event `self.Reset`
  (`PaperFlipbookComponent.SetPlaybackPositionInFrames` (`self.RenderComponent`) 0 false)
  (`PrimitiveComponent.SetCollisionResponseToChannel` (`self.Collision`) "ECC_Pawn" "ECR_Block")
  (goto _label :!via `Reset`))

(event `self.PlayerDetection.OnComponentBeginOverlap`
  (params (OverlappedComponent :type "PrimitiveComponent Object Reference") (OtherActor :type "Actor Object Reference") (OtherComp :type "PrimitiveComponent Object Reference") (OtherBodyIndex :type Integer) (bFromSweep :type Boolean) (SweepResult :type "HitResult Structure (by ref)"))
  (cast `/Game/Blueprints/Character/BP_Player` OtherActor)
  (`/Engine/EditorBlueprintResources/StandardMacros.DoOnce` false :!label _label
    (:`Completed`
      (`PaperFlipbookComponent.SetPlayRate` (`self.RenderComponent`) (`self.PlaySpeed`)))))

(fn `UserConstructionScript`
  (`parent.UserConstructionScript`))