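; BP_PlatformCloud is a cloud platform that lets pawns fall through after the player stands on it for a set duration.
; Player overlap with PlayerDetection opens a gate and starts a retriggerable delay, after which Collision switches its Pawn response to Overlap.
; Leaving the detection volume or calling Reset closes the gate, cancelling any pending drop, and restores blocking if it was disabled.
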(event `self.PlayerDetection.OnComponentBeginOverlap`
  (params (OverlappedComponent :type "PrimitiveComponent Object Reference") (OtherActor :type "Actor Object Reference") (OtherComp :type "PrimitiveComponent Object Reference") (OtherBodyIndex :type Integer) (bFromSweep :type Boolean) (SweepResult :type "HitResult Structure (by ref)"))
  (cast `/Game/Blueprints/Character/BP_Player` OtherActor)
  (`|ExecutionSequence`
    (:`then_0`
      (goto _label :!via `Open`))
    (:`then_1`
      (`KismetSystemLibrary.RetriggerableDelay` (`self.StandOnDuration`))
      (`/Engine/EditorBlueprintResources/StandardMacros.Gate` true :!label _label
        (:`Exit`
          (set `self.CollisionOff` true)
          (`PrimitiveComponent.SetCollisionResponseToChannel` (`self.Collision`) "ECC_Pawn" "ECR_Overlap"))))))

(event `self.PlayerDetection.OnComponentEndOverlap`
  (params (OverlappedComponent :type "PrimitiveComponent Object Reference") (OtherActor :type "Actor Object Reference") (OtherComp :type "PrimitiveComponent Object Reference") (OtherBodyIndex :type Integer))
  (cast `/Game/Blueprints/Character/BP_Player` OtherActor)
  (`|ExecutionSequence` :!label _label_2
    (:`then_0`
      (goto _label :!via `Close`))
    (:`then_1`
      (if (`self.CollisionOff`)
        (set `self.CollisionOff` false)
        (`PrimitiveComponent.SetCollisionResponseToChannel` (`self.Collision`) "ECC_Pawn" "ECR_Block")))))

(event `self.Reset`
  (goto _label_2))

(fn `UserConstructionScript`
  (`parent.UserConstructionScript`))