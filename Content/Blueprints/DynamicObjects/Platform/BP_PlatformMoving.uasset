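; BP_PlatformMoving is a 2D flipbook platform that moves through the XZ plane when its MovePlatform event fires.
; A timeline at PlaySpeed adds a world offset each update from its value, MovementDirection and MovementDistance, so movement accumulates.
; The same timeline value scrubs the flipbook frame.
; On finish the flipbook's play rate becomes PlaySpeed, and Tick zeroes it whenever the last frame is reached.
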(event `self.ReceiveBeginPlay`
  (`parent.ReceiveBeginPlay`))

(event `self.ReceiveTick`
  (params (DeltaSeconds :type "Float (single-precision)"))
  (bind _rendercomponent (`self.RenderComponent`))
  (`parent.ReceiveTick` DeltaSeconds)
  (if (== (`PaperFlipbookComponent.GetPlaybackPositionInFrames` _rendercomponent) (- (`PaperFlipbookComponent.GetFlipbookLengthInFrames` _rendercomponent) 1))
    (`PaperFlipbookComponent.SetPlayRate` (`self.RenderComponent`) 0.0)))

(event `MovePlatform`
  (bind _rendercomponent (`self.RenderComponent`))
  (`TimelineComponent.SetPlayRate` (`self.PlatformMovementTimer`) (`self.PlaySpeed`))
  (bind (_direction _value) (`Timeline|PlatformMovementTimer` :!via `PlayFromStart`)
    (:`Update`
      (bind (_returnvalue_x _returnvalue_y) (`KismetMathLibrary.BreakVector2D` (* _value (`self.MovementDirection`) (`self.MovementDistance`))))
      (`self.K2_AddActorWorldOffset` (`KismetMathLibrary.MakeVector` _returnvalue_x 0.0 _returnvalue_y))
      (`PaperFlipbookComponent.SetPlaybackPositionInFrames` _rendercomponent (`KismetMathLibrary.FFloor` (* _value 6.0)) false))
    (:`Finished`
      (`PaperFlipbookComponent.SetPlayRate` _rendercomponent (`self.PlaySpeed`)))))

(fn `UserConstructionScript`
  (`parent.UserConstructionScript`))